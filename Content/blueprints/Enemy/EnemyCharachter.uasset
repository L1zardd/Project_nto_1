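; Flipbook-based enemy character with back-and-forth patrol logic that reverses when a trace finds an obstacle.
; Each Tick picks the walk or idle flipbook from velocity and sets facing from the movement direction sign.
; Movement input is scaled by that sign, though its world direction is a zero vector.
; A forward visibility trace hit zeroes walk speed, waits, then restores speed and flips direction, gated by a resetting DoOnce.
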(event Custom|Animation%20Update
  ;[1 1 1] Anumation Update
  (Sprite|SetFlipbook (Variables|Default|GetSprite) (select (> (Math|Vector|VectorLength (Variables|/Script/Engine.MovementComponent|GetVelocity (Variables|Character|GetCharacterMovement))) 0.0) (Variables|Default|GetEnemy_walk_FB) (Variables|Default|GetEnemy_idle_FB))))

(event Custom|Movement%20Update
  (bind _returnvalue (Transformation|GetActorLocation))
  (Utilities|FlowControl|Sequence
    (:then_0
      (if (> (Variables|Default|GetMovemet%20Direction) 0.0)
        (Transformation|SetActorRotation "0, 0, 0")
        (else
          (Transformation|SetActorRotation "0.000000,180.000000,0.000000"))))
    (:then_1
      (Pawn|Input|AddMovementInput "0, 0, 0" (Variables|Default|GetMovemet%20Direction) false)
      (bind _returnvalue_2 (Collision|LineTraceByChannel _returnvalue (+ _returnvalue (* (Transformation|GetActorForwardVector) (Math|Vector|MakeVector 3e+02 0.0 0.0))) "TraceTypeQuery1" false 0 "None"))
      (if _returnvalue_2
        (Utilities|FlowControl|DoOnce false :!label _label
          (:Completed
            (Variables|/Script/Engine.CharacterMovementComponent|SetMaxWalkSpeed (Variables|Character|GetCharacterMovement) 0.0)
            (Utilities|FlowControl|Delay (Variables|Default|GetDuration))
            (Variables|/Script/Engine.CharacterMovementComponent|SetMaxWalkSpeed (Variables|Character|GetCharacterMovement) (Variables|Default|GetMax%20Walk%20Speed))
            (Variables|Default|SetMovemet%20Direction (* (Variables|Default|GetMovemet%20Direction) -1.0))
            (goto _label Reset)))))))

(event EventBeginPlay
  (Variables|/Script/Engine.CharacterMovementComponent|SetMaxWalkSpeed (Variables|Character|GetCharacterMovement) (Variables|Default|GetMax%20Walk%20Speed)))

(event EventTick
  (params (DeltaSeconds :type Float%20%28single-precision%29))
  (CallFunction|AnimationUpdate)
  (CallFunction|MovementUpdate))

(fn ConstructionScript)
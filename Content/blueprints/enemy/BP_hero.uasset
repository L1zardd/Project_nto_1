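; Player hero character for a side-scroller, moving along world X with double jump and hold-to-dash.
; Tick flips control yaw by velocity direction, dash raises walk speed and RunPlaRay, and jumps or ledge falls trigger the animation's jump node.
; BeginPlay creates the SVBP save if missing; pausing opens the game menu and saves the capsule location, which the R key restores.
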(event EventBeginPlay
  (bind _slot_name (Variables|Default|GetSlot%20Name))
  ;[1 1 1] Загрузка меню в игре и сохранение
  (bind _returnvalue (SaveGame|DoesSaveGameExist _slot_name))
  (if (not _returnvalue)
    (bind _returnvalue_2 (SaveGame|CreateSaveGameObject "/Game/blueprints/hero/SVBP.SVBP_C"))
    (SaveGame|SaveGametoSlot _returnvalue_2 _slot_name)))

(event EventOnJumped
  ;[1 1 1] Comment
  (Class|PaperZDAnimInstance|JumptoNode (Variables|/Script/PaperZD.PaperZDAnimationComponent|GetAnimInstance (Variables|Default|GetAnimationComponent)) "jumpaction" "None"))

(event EventOnWalkingOffLedge
  (params (PreviousFloorImpactNormal :type Vector%20%28by%20ref%29 :default "0, 0, 0") (PreviousFloorContactNormal :type Vector%20%28by%20ref%29 :default "0, 0, 0") (PreviousLocation :type Vector%20%28by%20ref%29 :default "0, 0, 0") (TimeDelta :type Float%20%28single-precision%29))
  ;[1 1 1] Comment
  (Class|PaperZDAnimInstance|JumptoNode (Variables|/Script/PaperZD.PaperZDAnimationComponent|GetAnimInstance (Variables|Default|GetAnimationComponent)) "jumpaction" "None"))

(event EventTick
  (params (DeltaSeconds :type Float%20%28single-precision%29))
  (bind _returnvalue (Pawn|GetController))
  (bind _returnvalue_2 (Pawn|GetController))
  ;[1 1 1] разворот
  (if (not (Variables|Default|GetIsMovementLock))
    (Math|Float|CompareFloat (.x (Variables|/Script/Engine.MovementComponent|GetVelocity (Variables|Character|GetCharacterMovement))) 0.0
      (:>
        (Utilities|IsValid _returnvalue
          (:Is%20Valid
            (Pawn|SetControlRotation _returnvalue (Math|Rotator|MakeRotator 0.0 0.0 0.0)))))
      (:<
        (Utilities|IsValid _returnvalue_2
          (:Is%20Valid
            (Pawn|SetControlRotation _returnvalue_2 (Math|Rotator|MakeRotator 0.0 0.0 1.8e+02))))))))

(event Input|ActionEvents|InputActionDASH
  (params (Key :type Key%20Structure))
  ;[1 1 1] ускорение
  (:Pressed
    (Variables|Default|SetRunPlaRay 1.5)
    (Variables|/Script/Engine.CharacterMovementComponent|SetMaxWalkSpeed (Variables|Character|GetCharacterMovement) 1e+03))
  (:Released
    (Variables|Default|SetRunPlaRay 1.0)
    (Variables|/Script/Engine.CharacterMovementComponent|SetMaxWalkSpeed (Variables|Character|GetCharacterMovement) 6e+02)))

(event Input|ActionEvents|InputActionJUMP
  (params (Key :type Key%20Structure))
  ;[1 1 1] прыжок
  (:Pressed
    (Variables|Default|SetJumpMaxHoldTime 0.2) ; высота прыжка
    (Variables|Default|SetJumpMaxCount 2) ; максимальное количество прыжков
    (Character|Jump) ; прыжок
  )
  (:Released
    (Character|StopJumping)))

(event Input|ActionEvents|InputActionPauseGame
  (params (Key :type Key%20Structure))
  (bind _returnvalue (Game|GetPlayerController 0))
  (bind _slot_name (Variables|Default|GetSlot%20Name))
  ;[1 1 1] Загрузка меню в игре и сохранение
  (:Pressed
    (Utilities|FlowControl|Sequence
      (:then_0
        (Game|SetGamePaused true)
        (Input|DisableInput _returnvalue)
        (bind _returnvalue_2 (UserInterface|CreateWidget "/Game/asets/widget/WDGameMenu.WDGameMenu_C" _returnvalue))
        (bind _output_get (Variables|Default|SetWD_Game_Menu _returnvalue_2))
        (UserInterface|Viewport|AddtoViewport _output_get 0)
        (Variables|/Script/Engine.PlayerController|SetbShowMouseCursor _returnvalue false)
        (Input|SetInputModeUIOnly _returnvalue 0 "DoNotLock" false))
      (:then_1
        (bind _returnvalue_3 (SaveGame|LoadGamefromSlot _slot_name))
        (bind _assvbp (Utilities|Casting|CastToSVBP _returnvalue_3))
        (Variables|/Game/blueprints/hero/SVBP.SVBP_C|SetLocation _assvbp (Transformation|GetWorldLocation (Variables|Default|GetCapsuleComponent)))
        (SaveGame|SaveGametoSlot _assvbp _slot_name)))))

(event Input|AxisEvents|InputAxisMove
  (params (AxisValue :type Float%20%28single-precision%29))
  ;[1 1 1] ходьба
  (if (not (Variables|Default|GetIsMovementLock))
    (Pawn|Input|AddMovementInput "1.000000,0.000000,0.000000" AxisValue false)))

(event Input|KeyboardEvents|R
  (params (Key :type Key%20Structure))
  ;[1 1 1] Загрузка меню в игре и сохранение
  (:Pressed
    (bind _returnvalue (SaveGame|LoadGamefromSlot (Variables|Default|GetSlot%20Name)))
    (bind _assvbp (Utilities|Casting|CastToSVBP _returnvalue))
    (Transformation|SetActorLocation (Variables|/Game/blueprints/hero/SVBP.SVBP_C|GetLocation _assvbp) false false)))

(fn ConstructionScript)